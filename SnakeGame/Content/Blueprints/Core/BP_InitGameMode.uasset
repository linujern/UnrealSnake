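; BP_InitGameMode is the startup game mode that hands the game off to the main menu.
; On BeginPlay it binds to the state machine subsystem's global state change event, waits briefly, then requests the Menu state.
; The change handler opens the main menu level for Menu and prints a red on-screen invalid-state message for any other state.
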(event `self.ReceiveBeginPlay`
  (add `StateMachineSubsystem.OnGlobalStateChanged` (subsystem `StateMachineSubsystem`) (delegate `OnGlobalStateChanged`))
  (`KismetSystemLibrary.Delay` 2.0)
  (`StateMachineSubsystem.ChangeState` (subsystem `StateMachineSubsystem`) "Menu"))

(event `OnGlobalStateChanged`
  (params (OldGlobalState :type "EGlobalState Enum" :default "Init") (NewGlobalState :type "EGlobalState Enum" :default "Init"))
  (if (`|EnumEquality` NewGlobalState "Menu")
    (`GameplayStatics.OpenLevelBySoftObjectPtr` "/Game/Levels/L_MainMenu.L_MainMenu")
    (else
      (`KismetSystemLibrary.PrintString` (`KismetStringLibrary.Concat_StrStr` (`|GetEnumeratorNameAsString` NewGlobalState) " : Invalid State") true true (struct :`R` 1.0 :`B` 0.016899 :`A` 1.0) 20.0))))

(fn `UserConstructionScript`)
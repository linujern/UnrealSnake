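; BP_PlayMode sets up a Snake play session and shows the Pause and Outro screens.
; On BeginPlay it caches BP_SnakeGameState, loads game data through the GameDataSubsystem and prints the apples needed per level.
; If a second snake agent is set, it creates another local player and offsets the two pawns to opposite sides.
; It then binds to the StateMachineSubsystem's global state changes to spawn the matching widget.
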(event `self.ReceiveBeginPlay`
  (`|ExecutionSequence`
    (:`then_0`
      (`self.Init`)
      ; If one agent only
      (if (not (`|EnumEquality` "None" (`SnakeGameState.GetSnakeAgent2` (`self.SnakeGameState`))))
        (`GameplayStatics.CreatePlayer` -1)
        (`self.K2_AddActorLocalOffset` (`GameplayStatics.GetPlayerPawn` 0) (0.0 -100.0 0.0) false false)
        (`self.K2_AddActorLocalOffset` (`GameplayStatics.GetPlayerPawn` 1) (0.0 100.0 0.0) false false)))
    (:`then_1`
      (add `StateMachineSubsystem.OnGlobalStateChanged` (subsystem `StateMachineSubsystem`) (delegate `OnGlobalStateChanged`)))))

(event `OnGlobalStateChanged`
  (params (OldGlobalState :type "EGlobalState Enum" :default "Init") (NewGlobalState :type "EGlobalState Enum" :default "Init"))
  (switch `EGlobalState` NewGlobalState
    (:`Pause`
      (bind _returnvalue (`|CreateWidget` "/Game/Blueprints/UI/WBP_Pause.WBP_Pause_C"))
      (`UserWidget.AddToViewport` _returnvalue 0))
    (:`Outro`
      (bind _returnvalue_2 (`|CreateWidget` "/Game/Blueprints/UI/WBP_Outro.WBP_Outro_C"))
      (`UserWidget.AddToViewport` _returnvalue_2 0))))

(fn `Init`
  (bind _asbp_snake_game_state (cast `/Game/Blueprints/Core/BP_SnakeGameState` (`GameplayStatics.GetGameState`))
    (:`then`
      (bind _output_get (set `self.SnakeGameState` _asbp_snake_game_state))
      (`GameDataSubsystem.LoadGameData` (subsystem `GameDataSubsystem`))
      (bind _returnvalue (`SnakeGameState.GetApplesPerLevel` _output_get))
      (`KismetSystemLibrary.PrintString` (`KismetStringLibrary.Concat_StrStr` (`KismetStringLibrary.Conv_IntToString` _returnvalue) " apples to complete")))
    (:`CastFailed`
      (`KismetSystemLibrary.PrintString` "NoSnakeGameState"))))

(fn `UserConstructionScript`)